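; Player controller for a two-team, turn-based tile tactics game that assigns a team and spawn on NewMap.
; On a player's turn, clicks drive movement, then an attack on an enemy or base; Space skips attacks.
; Game state holds turn, phase and base health; player state holds team, position and tiles in range.
; Range tiles are computed by index, then highlighted through line traces on the offset grid and custom depth.
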(event Custom|Begin%20Turn
  ;[1 1 1] Begin Move Phase
  (Utilities|FlowControl|Delay 1.0)
  (bind _asbp_game_state (Utilities|Casting|CastToBP_Game_State (Game|GetGameState)))
  (bind _asplayer_state_bp (Utilities|Casting|CastToplayer_state_BP (Variables|Default|GetPlayerState)))
  (if (Math|Boolean|Equal(Boolean) (Variables|/Game/_Blueprints/player_state_BP.player_state_BP_C|GetTeam _asplayer_state_bp) (Variables|/Game/_Blueprints/BP_Game_State.BP_Game_State_C|GetTeamToMove _asbp_game_state))
    (CallFunction|GetTilesinRange _asplayer_state_bp (Variables|/Game/_Blueprints/player_state_BP.player_state_BP_C|GetTile%20Index _asplayer_state_bp) (Variables|/Game/_Blueprints/player_state_BP.player_state_BP_C|GetRange _asplayer_state_bp))
    (CallFunction|HighlightTilesinRange _asplayer_state_bp true)))

(event Custom|switchTeam
  ;[1 1 1] Dev Tools
  ;;[1 1 1] Spacebar Swaps Team (on server)
  (bind _asplayer_state_bp (Utilities|Casting|CastToplayer_state_BP (Variables|Default|GetPlayerState)))
  (Variables|/Game/_Blueprints/player_state_BP.player_state_BP_C|SetTeam _asplayer_state_bp (not (Variables|/Game/_Blueprints/player_state_BP.player_state_BP_C|GetTeam _asplayer_state_bp)))
  (CallFunction|UpdateHUDMulticast))

(event Custom|Destroy%20Actor%20on%20client
  (params (Actor :type Actor%20Object%20Reference))
  ;[1 1 1] Destory actor
  (Utilities|IsValid Actor ; making sure its not done again if the guys already dead
    (:Is%20Valid
      (Actor|DestroyActor Actor))))

(event Custom|Destory%20Actor%20on%20server
  (params (Actor :type Actor%20Object%20Reference))
  ;[1 1 1] Destory actor
  (CallFunction|DestroyActoronClient Actor))

(event Custom|End%20game%20multicast
  (bind _asthird_person_character (Utilities|Casting|CastToThirdPersonCharacter (Game|GetPlayerCharacter 0)))
  (Default|EndGameServer _asthird_person_character))

(event Custom|Swap%20turn
  ;[1 1 1] Swap Turn
  (bind _asbp_game_state (Utilities|Casting|CastToBP_Game_State (Game|GetGameState)))
  (Variables|/Game/_Blueprints/BP_Game_State.BP_Game_State_C|SetTeamToMove _asbp_game_state (not (Variables|/Game/_Blueprints/BP_Game_State.BP_Game_State_C|GetTeamToMove _asbp_game_state))))

(event Custom|server%20begin%20turn
  ;[1 1 1] display HUD & set team
  (CallFunction|BeginTurn self))

(event Custom|Attack
  (bind _array (Utilities|Array|MakeArray "ObjectTypeQuery1" "ObjectTypeQuery3" "ObjectTypeQuery2" "ObjectTypeQuery1"))
  (bind _self self)
  (bind _hitresult (Class|PlayerController|GetHitResultUnderCursorforObjects _self _array true))
  ;[1 1 1] Attack
  (bind _aspawn (Utilities|Casting|CastToPawn (.hitactor _hitresult))
    (:then
      (bind _asplayer_state_bp (Utilities|Casting|CastToplayer_state_BP (Variables|/Script/Engine.Pawn|GetPlayerState _aspawn)))
      (bind _asplayer_state_bp_2 (Utilities|Casting|CastToplayer_state_BP (Variables|Default|GetPlayerState)))
      (if (Math|Boolean|Equal(Boolean) (Variables|/Game/_Blueprints/player_state_BP.player_state_BP_C|GetTeam _asplayer_state_bp_2) (Variables|/Game/_Blueprints/player_state_BP.player_state_BP_C|GetTeam _asplayer_state_bp))
        (Development|PrintString "You can't attack yourself")
        (else
          (for _array_element (Variables|/Game/_Blueprints/player_state_BP.player_state_BP_C|GetTilesInRange _asplayer_state_bp_2)
            (if (Class|KismetMathLibrary|EqualIntPointIntPoint _array_element (Variables|/Game/_Blueprints/player_state_BP.player_state_BP_C|GetTile%20Index _asplayer_state_bp))
              (Variables|Default|SetIn%20range (Class|KismetMathLibrary|EqualIntPointIntPoint _array_element (Variables|/Game/_Blueprints/player_state_BP.player_state_BP_C|GetTile%20Index _asplayer_state_bp)))))
          (if (Variables|Default|GetIn%20range)
            (CallFunction|EndAttackPhase)
            (CallFunction|TakeDamage 5e+01 _asplayer_state_bp)
            (CallFunction|HealthCheck _asplayer_state_bp)
            (Variables|Default|SetIn%20range false)
            (else
              (Development|PrintString "Enemy not in range"))))))
    (:CastFailed
      (Utilities|Casting|CastToBP_Base (.hitactor _hitresult)
        (:then
          (CallFunction|AttackBase1))
        (:CastFailed
          (Utilities|Casting|CastToBP_Base2 (.hitactor _hitresult))
          (CallFunction|AttackBase2))))))

(event Custom|End%20Attack%20Phase
  ;[1 1 1] End Attack Phase
  (bind _asbp_game_state (Utilities|Casting|CastToBP_Game_State (Game|GetGameState)))
  (Variables|/Game/_Blueprints/BP_Game_State.BP_Game_State_C|SetAttack%20Phase _asbp_game_state false)
  (bind _asplayer_state_bp (Utilities|Casting|CastToplayer_state_BP (Variables|Default|GetPlayerState)))
  (CallFunction|HighlightTilesinRange _asplayer_state_bp false)
  (CallFunction|SwapTurn))

(event Custom|Begin%20Attack%20Phase
  ;[1 1 1] Begin Attack Phase
  (bind _asbp_game_state (Utilities|Casting|CastToBP_Game_State (Game|GetGameState)))
  (Variables|/Game/_Blueprints/BP_Game_State.BP_Game_State_C|SetAttack%20Phase _asbp_game_state true)
  (bind _asplayer_state_bp (Utilities|Casting|CastToplayer_state_BP (Variables|Default|GetPlayerState)))
  (CallFunction|GetTilesinRange _asplayer_state_bp (Variables|/Game/_Blueprints/player_state_BP.player_state_BP_C|GetTile%20Index _asplayer_state_bp) 3)
  (CallFunction|HighlightTilesinRange _asplayer_state_bp true))

(event Custom|Server%20Set%20Tile%20Index
  (params (NewParam :type Int%20Point%20Structure) (NewParam2 :type Player%20State%20BP%20Object%20Reference))
  ;[1 1 1] Movement
  (Variables|/Game/_Blueprints/player_state_BP.player_state_BP_C|SetTile%20Index NewParam2 NewParam))

(event Custom|Update%20HUD%20Multicast
  ;[1 1 1] update HUD multicast
  (bind _asthird_person_character (Utilities|Casting|CastToThirdPersonCharacter (Game|Player|GetPlayerPawn 0)))
  (Default|CallUpdateHUD _asthird_person_character))

(event Custom|SetTeam
  ;[1 1 1] Sets team (player state) to team to join (game state)
  (bind _asplayer_state_bp (Utilities|Casting|CastToplayer_state_BP (Variables|Default|GetPlayerState)))
  (bind _asbp_game_state (Utilities|Casting|CastToBP_Game_State (Game|GetGameState)))
  (Variables|/Game/_Blueprints/player_state_BP.player_state_BP_C|SetTeam _asplayer_state_bp (Variables|/Game/_Blueprints/BP_Game_State.BP_Game_State_C|GetTeamToJoin _asbp_game_state))
  (CallFunction|UpdateHUDMulticast))

(event Custom|Attack%20Base%202
  ;[1 1 1] Base Attack
  (bind _asplayer_state_bp (Utilities|Casting|CastToplayer_state_BP (Variables|Default|GetPlayerState)))
  (if (Variables|/Game/_Blueprints/player_state_BP.player_state_BP_C|GetTeam _asplayer_state_bp)
    (Development|PrintString "You can't attack your own base")
    (else
      (bind _inrange (CallFunction|IsBase2inRange))
      (if _inrange
        (bind _asbp_game_state (Utilities|Casting|CastToBP_Game_State (Game|GetGameState)))
        (bind _output_get (Variables|/Game/_Blueprints/BP_Game_State.BP_Game_State_C|SetBase2Health _asbp_game_state (- (Variables|/Game/_Blueprints/BP_Game_State.BP_Game_State_C|GetBase2Health _asbp_game_state) 50)))
        (Development|PrintString (Utilities|String|Append "Base Health: " (Utilities|String|ToString(Integer) _output_get)))
        (if (<= _output_get 0)
          (bind _asthird_person_character (Utilities|Casting|CastToThirdPersonCharacter (Game|GetPlayerCharacter 0)))
          (Default|EndGameServer _asthird_person_character)
          (else
            (CallFunction|EndAttackPhase)))
        (else
          (Development|PrintString "Base not in range"))))))

(event Custom|Attack%20Base%201
  ;[1 1 1] Base Attack
  (bind _asplayer_state_bp (Utilities|Casting|CastToplayer_state_BP (Variables|Default|GetPlayerState)))
  (if (Variables|/Game/_Blueprints/player_state_BP.player_state_BP_C|GetTeam _asplayer_state_bp)
    (bind _inrange (CallFunction|IsBase1inRange))
    (if _inrange
      (bind _asbp_game_state (Utilities|Casting|CastToBP_Game_State (Game|GetGameState)))
      (bind _output_get (Variables|/Game/_Blueprints/BP_Game_State.BP_Game_State_C|SetBase1Health _asbp_game_state (- (Variables|/Game/_Blueprints/BP_Game_State.BP_Game_State_C|GetBase1Health _asbp_game_state) 50)))
      (Development|PrintString (Utilities|String|Append "Base Health: " (Utilities|String|ToString(Integer) _output_get)))
      (if (<= _output_get 0)
        (bind _asthird_person_character (Utilities|Casting|CastToThirdPersonCharacter (Game|GetPlayerCharacter 0)))
        (Default|EndGameServer _asthird_person_character)
        (else
          (CallFunction|EndAttackPhase)))
      (else
        (Development|PrintString "Base not in range")))
    (else
      (Development|PrintString "You can't attack your own base"))))

(event Custom|Multi%20print%20health
  (params (NewParam :type Float%20%28single-precision%29))
  (Development|PrintString "Player hit!")
  (Development|PrintString (Utilities|String|ToString(Text) (Utilities|Text|FormatText "Health: {hp}" NewParam))))

(event Custom|Send%20to%20Spawn
  (params (Player%20State :type Player%20State%20BP%20Object%20Reference))
  ;[1 1 1] send to spawn
  (if (Variables|/Game/_Blueprints/player_state_BP.player_state_BP_C|GetTeam Player%20State)
    (Variables|/Game/_Blueprints/player_state_BP.player_state_BP_C|SetSpawnpoint Player%20State "448.000000,4805.000000,150.000000")
    (Variables|/Game/_Blueprints/player_state_BP.player_state_BP_C|SetTile%20Index Player%20State (Utilities|Struct|MakeIntPoint 2 31))
    (else
      (Variables|/Game/_Blueprints/player_state_BP.player_state_BP_C|SetSpawnpoint Player%20State "5524.000000,310.000000,250.000000")
      (Variables|/Game/_Blueprints/player_state_BP.player_state_BP_C|SetTile%20Index Player%20State (Utilities|Struct|MakeIntPoint 31 2))))
  (Transformation|SetActorLocation (Variables|/Script/Engine.PlayerState|GetPawnPrivate Player%20State) (Variables|/Game/_Blueprints/player_state_BP.player_state_BP_C|GetSpawnpoint Player%20State) false false))

(event Custom|Take%20damage
  (params (attack :type Float%20%28single-precision%29) (other%20player :type Player%20State%20BP%20Object%20Reference))
  ;[1 1 1] Deal damage
  (bind _output_get (Variables|/Game/_Blueprints/player_state_BP.player_state_BP_C|SetStats other%20player (Utilities|Struct|MakeStats 1e+02 1e+02 1e+02 1e+02 2 2 2 (- (.health (Variables|/Game/_Blueprints/player_state_BP.player_state_BP_C|GetStats other%20player)) attack) 0)))
  (CallFunction|MultiPrintHealth (.health _output_get)))

(event Custom|Movement
  (bind _self self)
  (bind _hitresult (Game|Player|GetHitResultUnderCursorbyChannel _self "TraceTypeQuery1" true))
  ;[1 1 1] Movement
  (bind _astile_bp (Utilities|Casting|CastToTile_BP (.hitactor _hitresult)))
  (Utilities|Casting|CastToWater_Tile_BP _astile_bp
    (:then
      (Development|PrintString "Cant move to water tile"))
    (:CastFailed
      (Utilities|Casting|CastToCliff_Tile_BP _astile_bp
        (:then
          (Development|PrintString "Can't move to cliff tile"))
        (:CastFailed
          (Utilities|Casting|CastToBase_Tile_BP (.hitactor _hitresult)
            (:then
              (Development|PrintString "Can't move to base tile"))
            (:CastFailed
              (bind _asplayer_state_bp (Utilities|Casting|CastToplayer_state_BP (Variables|Default|GetPlayerState)))
              (for _array_element (Variables|/Game/_Blueprints/player_state_BP.player_state_BP_C|GetTilesInRange _asplayer_state_bp)
                (if (Class|KismetMathLibrary|EqualIntPointIntPoint _array_element (Variables|/Script/MbR_eSports.Tile|GetTileIndex _astile_bp))
                  (Variables|Default|SetIn%20range (Class|KismetMathLibrary|EqualIntPointIntPoint _array_element (Variables|/Script/MbR_eSports.Tile|GetTileIndex _astile_bp)))))
              (if (Variables|Default|GetIn%20range)
                (Variables|/Game/_Blueprints/player_state_BP.player_state_BP_C|SetTile%20Index _asplayer_state_bp (Variables|/Script/MbR_eSports.Tile|GetTileIndex _astile_bp))
                (CallFunction|HighlightTilesinRange self _asplayer_state_bp false)
                (Variables|Default|SetIn%20range false)
                (bind _asthird_person_character (Utilities|Casting|CastToThirdPersonCharacter (Game|GetPlayerCharacter 0)))
                (Default|MoveCharacter _asthird_person_character (Transformation|GetActorLocation _astile_bp))
                (CallFunction|BeginAttackPhase)
                (CallFunction|ServerSetTileIndex (Variables|/Script/MbR_eSports.Tile|GetTileIndex _astile_bp) _asplayer_state_bp)
                (else
                  (Development|PrintString "Tile not in range"))))))))))

(event Custom|Health%20Check
  (params (other%20player :type Player%20State%20BP%20Object%20Reference))
  ;[1 1 1] Health check
  (if (<= (Math|Float|Truncate (.health (Variables|/Game/_Blueprints/player_state_BP.player_state_BP_C|GetStats other%20player))) 0)
    (CallFunction|EndGameMulticast)))

(event EventBeginPlay
  ;[1 1 1] display HUD & set team
  (bind _returnvalue (Game|GetCurrentLevelName true))
  (if (Utilities|Enum|Equal(Enum) _returnvalue "NewMap")
    (Utilities|FlowControl|Delay 0.2)
    (CallFunction|SetTeam self)
    (bind _asplayer_state_bp (Utilities|Casting|CastToplayer_state_BP (Variables|Default|GetPlayerState)))
    (CallFunction|SendtoSpawn self _asplayer_state_bp)
    (CallFunction|ServerBeginTurn)))

(event Input|KeyboardEvents|SpaceBar
  (params (Key :type Key%20Structure :default "None"))
  ;[1 1 1] pass attack
  (:Pressed
    (bind _asbp_game_state (Utilities|Casting|CastToBP_Game_State (Game|GetGameState)))
    (if (Variables|/Game/_Blueprints/BP_Game_State.BP_Game_State_C|GetAttack%20Phase _asbp_game_state)
      (bind _isturn (CallFunction|IsTurn))
      (if _isturn
        (Development|PrintString "Attack skipped")
        (CallFunction|EndAttackPhase)))))

(event Input|KeyboardEvents|SpaceBar
  (params (Key :type Key%20Structure :default "None"))
  ;[1 1 1] Dev Tools
  ;;[1 1 1] Spacebar Swaps Team (on server)
)

(event Input|KeyboardEvents|Backspace
  (params (Key :type Key%20Structure :default "None"))
  ;[1 1 1] Dev Tools
  ;;[1 1 1] force turn skip
)

(event Input|KeyboardEvents|1
  (params (Key :type Key%20Structure :default "None"))
  ;[1 1 1] Dev Tools
  ;;[1 1 1] Tab prints teams, ID's and team to move
  (:Pressed
    (bind _asbp_game_state (Utilities|Casting|CastToBP_Game_State (Game|GetGameState)))
    (if (Variables|/Game/_Blueprints/BP_Game_State.BP_Game_State_C|GetTeamToMove _asbp_game_state)
      (Development|PrintString "Blue Teams Turn")
      (else
        (Development|PrintString "Red Teams Turn")))
    (bind _asplayer_state_bp (Utilities|Casting|CastToplayer_state_BP (Variables|Default|GetPlayerState)))
    (if (Variables|/Game/_Blueprints/player_state_BP.player_state_BP_C|GetTeam _asplayer_state_bp)
      (Development|PrintString "Your team: Blue Team")
      (else
        (Development|PrintString "Your team: Red Team")))))

(event Input|MouseEvents|LeftMouseButton
  (params (Key :type Key%20Structure :default "None"))
  ;[1 1 1] Player Input
  (:Pressed
    (bind _isturn (CallFunction|IsTurn))
    (if _isturn
      (bind _asbp_game_state (Utilities|Casting|CastToBP_Game_State (Game|GetGameState)))
      (if (Variables|/Game/_Blueprints/BP_Game_State.BP_Game_State_C|GetAttack%20Phase _asbp_game_state)
        (CallFunction|Attack)
        (else
          (CallFunction|Movement))))))

(fn ConstructionScript)

(fn DisplayHUD
  (if (Pawn|IsLocalPlayerController)
    (bind _returnvalue (UserInterface|CreateWidget "/Game/_Blueprints/HUD.HUD_C"))
    (bind _output_get (Variables|Default|SetHUD _returnvalue))
    (UserInterface|Viewport|AddtoViewport _output_get 0)))

(fn IsTurn
  (bind _asbp_game_state (Utilities|Casting|CastToBP_Game_State (Game|GetGameState)))
  (bind _asplayer_state_bp (Utilities|Casting|CastToplayer_state_BP (Variables|Default|GetPlayerState)))
  (return (Math|Boolean|Equal(Boolean) (Variables|/Game/_Blueprints/player_state_BP.player_state_BP_C|GetTeam _asplayer_state_bp) (Variables|/Game/_Blueprints/BP_Game_State.BP_Game_State_C|GetTeamToMove _asbp_game_state))))

(fn GetTilesinRange
  (params (PlayerState :type Player%20State%20BP%20Object%20Reference) (CurrentPoint :type Int%20Point%20Structure) (Range :type Integer))
  (bind _returnvalue (- (.y CurrentPoint) Range))
  (bind _returnvalue_2 (+ (.y CurrentPoint) Range))
  (bind _tilesinrange (Variables|/Game/_Blueprints/player_state_BP.player_state_BP_C|GetTilesInRange PlayerState))
  (Utilities|Array|Clear _tilesinrange)
  (Variables|Default|SetArrayElement 0)
  (bind _output_get (Variables|Default|Seti (* Range -1)))
  (for _index (range (- (.x CurrentPoint) Range) (+ (.x CurrentPoint) Range))
    (if (< _output_get 1)
      (for _index_2 (range (- _returnvalue _output_get) (+ _returnvalue_2 _output_get))
        (Utilities|Array|SetArrayElem _tilesinrange (Variables|Default|GetArrayElement) (Utilities|Struct|MakeIntPoint _index _index_2) true)
        (Variables|Default|SetArrayElement (+ (Variables|Default|GetArrayElement) 1)))
      (else
        (for _index_3 (range (+ _returnvalue _output_get) (- _returnvalue_2 _output_get))
          (Utilities|Array|SetArrayElem _tilesinrange (Variables|Default|GetArrayElement) (Utilities|Struct|MakeIntPoint _index _index_3) true)
          (Variables|Default|SetArrayElement (+ (Variables|Default|GetArrayElement) 1)))))
    (Variables|Default|Seti (+ (Variables|Default|Geti) 1))))

(fn HighlightTilesinRange
  (params (PlayerState :type Player%20State%20BP%20Object%20Reference) (Highlight :type Boolean))
  (for _array_element (Variables|/Game/_Blueprints/player_state_BP.player_state_BP_C|GetTilesInRange PlayerState)
    (bind _output_get (Variables|Default|SetLineTraceX (* (Math|Conversions|ToFloat(Integer) (.x _array_element)) 178.199997)))
    (Variables|Default|SetLineTraceY (* (Math|Conversions|ToFloat(Integer) (.y _array_element)) 155.0))
    (if (== (Math|Float|%(Float) (Math|Conversions|ToFloat(Integer) (.y _array_element)) 2.0) 1.0)
      (Variables|Default|SetLineTraceX (+ 89.099998 _output_get 0.0)))
    (bind _outhit (Collision|LineTraceByChannel (Math|Vector|MakeVector (Variables|Default|GetLineTraceX) (Variables|Default|GetLineTraceY) 2e+02) (Math|Vector|MakeVector (Variables|Default|GetLineTraceX) (Variables|Default|GetLineTraceY) -2e+02) "TraceTypeQuery1" false 0 "None"))
    (if (.bblockinghit _outhit)
      (Utilities|Casting|CastToTile_BP (.hitactor _outhit))
      (Utilities|Casting|CastToWater_Tile_BP (.hitactor _outhit)
        (:CastFailed
          (Utilities|Casting|CastToCliff_Tile_BP (.hitactor _outhit)
            (:CastFailed
              (Utilities|Casting|CastToBase_Tile_BP (.hitactor _outhit)
                (:CastFailed
                  (Rendering|SetRenderCustomDepth (Actor|GetComponentbyClass (.hitactor _outhit) "/Script/Engine.StaticMeshComponent") Highlight))))))))))

(fn IsBase1inRange
  (bind _asplayer_state_bp (Utilities|Casting|CastToplayer_state_BP (Variables|Default|GetPlayerState)))
  (for _array_element (Variables|/Game/_Blueprints/player_state_BP.player_state_BP_C|GetTilesInRange _asplayer_state_bp)
    (if (Math|Boolean|ORBoolean (Class|KismetMathLibrary|EqualIntPointIntPoint _array_element (Utilities|Struct|MakeIntPoint 31 1)) (Class|KismetMathLibrary|EqualIntPointIntPoint _array_element (Utilities|Struct|MakeIntPoint 30 1)) (Class|KismetMathLibrary|EqualIntPointIntPoint _array_element (Utilities|Struct|MakeIntPoint 30 0)))
      (return true)))
  (return false))

(fn IsBase2inRange
  (bind _asplayer_state_bp (Utilities|Casting|CastToplayer_state_BP (Variables|Default|GetPlayerState)))
  (for _array_element (Variables|/Game/_Blueprints/player_state_BP.player_state_BP_C|GetTilesInRange _asplayer_state_bp)
    (if (Math|Boolean|ORBoolean (Class|KismetMathLibrary|EqualIntPointIntPoint _array_element (Utilities|Struct|MakeIntPoint 1 31)) (Class|KismetMathLibrary|EqualIntPointIntPoint _array_element (Utilities|Struct|MakeIntPoint 1 30)) (Class|KismetMathLibrary|EqualIntPointIntPoint _array_element (Utilities|Struct|MakeIntPoint 0 30)))
      (return true)))
  (return false))